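; Vivern enemy NPC that attacks the player, shows a name and health bar, and counts toward kill quests.
; Three hit boxes damage the player on overlap while Attacking is set, clearing the flag on each hit.
; Any incoming damage removes fixed HP and updates the bar widget.
; At zero HP it decrements matching player quests (outside the Died guard), then once plays death, flags the AI blackboard and destroys itself after a delay.
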(event OnComponentBeginOverlap(Box2)
  (params (OverlappedComponent :type Primitive%20Component%20Object%20Reference) (OtherActor :type Actor%20Object%20Reference) (OtherComp :type Primitive%20Component%20Object%20Reference) (OtherBodyIndex :type Integer) (bFromSweep :type Boolean) (SweepResult :type Hit%20Result%20Structure%20%28by%20ref%29))
  (bind _returnvalue (Game|Player|GetPlayerPawn 0))
  (if (== OtherActor _returnvalue)
    (if (Variables|Default|GetAttacking)
      (Variables|Default|SetAttacking false)
      (Game|Damage|ApplyDamage _returnvalue 5e+01 0 0))))

(event OnComponentBeginOverlap(Box1)
  (params (OverlappedComponent :type Primitive%20Component%20Object%20Reference) (OtherActor :type Actor%20Object%20Reference) (OtherComp :type Primitive%20Component%20Object%20Reference) (OtherBodyIndex :type Integer) (bFromSweep :type Boolean) (SweepResult :type Hit%20Result%20Structure%20%28by%20ref%29))
  (bind _returnvalue (Game|Player|GetPlayerPawn 0))
  (if (== OtherActor _returnvalue)
    (if (Variables|Default|GetAttacking)
      (Variables|Default|SetAttacking false)
      (Game|Damage|ApplyDamage _returnvalue 2e+01 0 0))))

(event OnComponentBeginOverlap(Box3)
  (params (OverlappedComponent :type Primitive%20Component%20Object%20Reference) (OtherActor :type Actor%20Object%20Reference) (OtherComp :type Primitive%20Component%20Object%20Reference) (OtherBodyIndex :type Integer) (bFromSweep :type Boolean) (SweepResult :type Hit%20Result%20Structure%20%28by%20ref%29))
  (bind _returnvalue (Game|Player|GetPlayerPawn 0))
  (if (== OtherActor _returnvalue)
    (if (Variables|Default|GetAttacking)
      (Variables|Default|SetAttacking false)
      (Game|Damage|ApplyDamage _returnvalue 2e+01 0 0))))

(event EventBeginPlay
  (bind _hp (Variables|Default|GetHP))
  (Variables|/Game/NPC/Other/HP.HP_C|SetMaxHP _hp (Variables|Default|GetHealth))
  (Default|SetHP _hp)
  (bind _asactor_bar (Utilities|Casting|CastToActorBar (Variables|/Script/Engine.ChildActorComponent|GetChildActor (Variables|Default|GetActorBar))))
  (Variables|/Game/NPC/Other/ActorBar.ActorBar_C|SetNPCName _asactor_bar (Variables|Default|GetNameNPC))
  (Default|SetName _asactor_bar))

(event Game|Damage|EventAnyDamage
  (params (Damage :type Float%20%28single-precision%29) (DamageType :type Damage%20Type%20Object%20Reference) (InstigatedBy :type Controller%20Object%20Reference) (DamageCauser :type Actor%20Object%20Reference))
  (bind _hp (Variables|Default|GetHP))
  (bind _hp_2 (Variables|/Game/NPC/Other/HP.HP_C|GetHP _hp))
  (Default|GetDamage _hp 3.0)
  (bind _asactor_bar (Utilities|Casting|CastToActorBar (Variables|/Script/Engine.ChildActorComponent|GetChildActor (Variables|Default|GetActorBar))))
  (bind _asnpcbar (Utilities|Casting|CastToNPCBar (UserInterface|GetWidget (Variables|/Game/NPC/Other/ActorBar.ActorBar_C|GetWidget _asactor_bar))))
  (Progress|SetPercent (Variables|/Game/NPC/Other/NPCBar.NPCBar_C|GetProgressBar_0 _asnpcbar) (/ _hp_2 (Variables|/Game/NPC/Other/HP.HP_C|GetMaxHP _hp)))
  (if (<= _hp_2 0.0)
    (bind _aschar_bp (Utilities|Casting|CastToCharBP (Game|Player|GetPlayerPawn 0)))
    (bind (_array_element _array_index) (Utilities|Array|ForEachLoopwithBreak (Variables|/Game/BluePrints/CharBP.CharBP_C|GetQuestStruckt _aschar_bp) :!label _label)
      (:LoopBody
        (for _array_element_2 (.enemy (.Quest (Utilities|Struct|BreakPlayerQuestStruct _array_element)))
          (if (== _array_element_2 (Utilities|GetClass self))
            (if (<= (- (.num (.Quest (Utilities|Struct|BreakPlayerQuestStruct _array_element))) 1) 0)
              (Variables|Default|SetKilled true)
              (else
                (Variables|Default|SetKilled false)))
            (|SetBy-RefVar (Utilities|Array|Get(acopy) (Variables|/Game/BluePrints/CharBP.CharBP_C|GetQuestStruckt _aschar_bp) _array_index) (Utilities|Struct|MakePlayerQuestStruct (Variables|Default|GetKilled) (Utilities|Struct|MakeNPCQuestStruct (.name (.Quest (Utilities|Struct|BreakPlayerQuestStruct _array_element))) (- (.num (.Quest (Utilities|Struct|BreakPlayerQuestStruct _array_element))) 1) (.enemy (.Quest (Utilities|Struct|BreakPlayerQuestStruct _array_element))) (.requester (.Quest (Utilities|Struct|BreakPlayerQuestStruct _array_element))) (.enemyname (.Quest (Utilities|Struct|BreakPlayerQuestStruct _array_element)))) (.NameOfRequester (Utilities|Struct|BreakPlayerQuestStruct _array_element))))
            (goto _label Break))))
      (:Completed
        (if (not (Variables|Default|GetDied))
          (Components|Animation|PlayAnimation (Variables|Character|GetMesh) "/Game/NPC/Vivern/AI/VivDeath.VivDeath" false)
          (Input|DisableInput 0)
          (bind _output_get (Variables|Default|SetDied true))
          (AI|Components|Blackboard|SetValueasBool (AI|GetBlackboard 0) (Utilities|Name|MakeLiteralName "Die") _output_get)
          (Utilities|FlowControl|Delay 3.3)
          (Actor|DestroyActor))))))

(fn ConstructionScript)